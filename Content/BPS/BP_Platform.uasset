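; BP_Platform is a multi-mode platform whose PlatformType makes it movable, a teleporter or a launcher.
; The construction script picks the matching mesh and moves the Sphere marker to PositionControlPoint.
; Movable platforms use InterpToMovement between their start and that point.
; On box overlap, teleporters send the actor to the Sphere, while launchers pass it a vector from the Arrow's direction and size via LauncherMessage.
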(event OnComponentBeginOverlap(Box)
  (params (OverlappedComponent :type Primitive%20Component%20Object%20Reference) (OtherActor :type Actor%20Object%20Reference) (OtherComp :type Primitive%20Component%20Object%20Reference) (OtherBodyIndex :type Integer) (bFromSweep :type Boolean) (SweepResult :type Hit%20Result%20Structure%20%28by%20ref%29))
  (switch Utilities|FlowControl|Switch|SwitchonE_PlatformType (Variables|Default|GetPlatformType)
    (:NewEnumerator1
      (Transformation|Teleport OtherActor (Transformation|GetWorldLocation (Variables|Default|GetSphere)) "0, 0, 0"))
    (:NewEnumerator2
      (Class|BPPlayerInteractions|Launcher(Message) OtherActor (* (Math|Vector|GetForwardVector (Variables|/Script/Engine.SceneComponent|GetRelativeRotation (Variables|Default|GetArrow))) (* (Variables|/Script/Engine.ArrowComponent|GetArrowSize (Variables|Default|GetArrow)) 1e+03))))))

(event EventBeginPlay
  (bind _interptomovement (Variables|Default|GetInterpToMovement))
  (if (Utilities|Enum|Equal(Enum) (Variables|Default|GetPlatformType) "NewEnumerator0")
    (Components|Activation|Activate (Variables|Default|GetInterpToMovement) true)
    (Variables|/Script/Engine.InterpToMovementComponent|SetDuration _interptomovement (Variables|Default|GetMovableDuration))
    (Class|InterptoMovementComponent|AddControlPointPosition _interptomovement "0, 0, 0" true)
    (Class|InterptoMovementComponent|AddControlPointPosition _interptomovement (Variables|Default|GetPosition%20Control%20Point) true)
    (Class|InterptoMovementComponent|FinaliseControlPoints _interptomovement)))

(fn ConstructionScript
  (bind _platformmesh (Variables|Default|GetPlatformMesh))
  (Components|StaticMesh|SetStaticMesh (Variables|Debug|GetStaticMeshComponent) (Utilities|Select :Index (Variables|Default|GetPlatformType) :NewEnumerator0 (Utilities|Array|Get(acopy) _platformmesh) :NewEnumerator1 (Utilities|Array|Get(acopy) _platformmesh 1) :NewEnumerator2 (Utilities|Array|Get(acopy) _platformmesh 2)))
  (Transformation|SetRelativeLocation (Variables|Default|GetSphere) (Variables|Default|GetPosition%20Control%20Point) false false))