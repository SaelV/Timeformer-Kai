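; BP_COINS is a coin pickup with a Value that also sets its appearance.
; The construction script picks the static mesh from the MESH array according to Value.
; On BeginPlay, a short random delay precedes activating RotatingMovement, which staggers the spin between coins.
; Mesh overlap sends AddCoinMessage with Value and itself to the other actor, and the coin does not destroy itself here.
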(event OnComponentBeginOverlap(StaticMesh)
  (params (OverlappedComponent :type Primitive%20Component%20Object%20Reference) (OtherActor :type Actor%20Object%20Reference) (OtherComp :type Primitive%20Component%20Object%20Reference) (OtherBodyIndex :type Integer) (bFromSweep :type Boolean) (SweepResult :type Hit%20Result%20Structure%20%28by%20ref%29))
  (Class|BPPlayerInteractions|AddCoin(Message) OtherActor (Variables|Default|GetValue) self))

(event EventBeginPlay
  (Utilities|FlowControl|Delay (Math|Random|RandomFloatinRange 0.0 0.3))
  (Components|Activation|Activate (Variables|Default|GetRotatingMovement) false))

(event Collision|EventActorBeginOverlap
  (params (OtherActor :type Actor%20Object%20Reference)))

(event EventTick
  (params (DeltaSeconds :type Float%20%28single-precision%29)))

(fn ConstructionScript
  (bind _mesh (Variables|Default|GetMESH))
  (bind _output (Utilities|Array|Get(acopy) _mesh))
  (Components|StaticMesh|SetStaticMesh (Variables|Default|GetStaticMesh) (Utilities|Select :Index (Variables|Default|GetValue) :Option%200 _output :Option%201 _output :Option%202 (Utilities|Array|Get(acopy) _mesh 1) :Option%203 (Utilities|Array|Get(acopy) _mesh 2))))