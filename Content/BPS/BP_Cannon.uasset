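; BP_Cannon is a cannon that automatically and continuously fires BP_BULLET actors from its muzzle.
; A timeline, played at PlayRate from BeginPlay and restarted whenever it finishes, animates the cannon's scale and fires Shoot events.
; A looping MultiGate alternates those events between a pull sound and a push sound paired with a bullet spawn at the muzzle's location and rotation.
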(event EventBeginPlay
  (bind _muzzle (Variables|Default|GetMuzzle))
  (bind _returnvalue (Transformation|GetWorldLocation _muzzle))
  (Components|Timeline|SetPlayRate (Variables|Default|GetShootTimeline) (Variables|Default|GetPlayRate))
  (bind _scalemod (Timeline|ShootTimeline Play)
    (:Update
      (Transformation|SetRelativeScale3D (Variables|Default|GetCannon) (Math|Conversions|ToVector(Float) _scalemod)))
    (:Finished
      (Timeline|ShootTimeline PlayFromStart))
    (:Shoot
      (Utilities|FlowControl|MultiGate false true -1
        (:Out%200
          (Audio|PlaySoundatLocation "/Engine/VREditor/Sounds/UI/Laser_Pull.Laser_Pull" _returnvalue "0, 0, 0" 1.0 1.0 0.0 0 0 0 0))
        (:Out%201
          (Audio|PlaySoundatLocation "/Engine/VREditor/Sounds/UI/Laser_Push.Laser_Push" _returnvalue "0, 0, 0" 1.0 1.0 0.0 0 0 0 0)
          (Game|SpawnActorfromClass "/Game/BPS/BP_BULLET.BP_BULLET_C" (Math|Transform|MakeTransform _returnvalue (Transformation|GetWorldRotation _muzzle) "1.000000,1.000000,1.000000") "Undefined" "MultiplyWithRoot" 0 0))))))

(event Collision|EventActorBeginOverlap
  (params (OtherActor :type Actor%20Object%20Reference)))

(event EventTick
  (params (DeltaSeconds :type Float%20%28single-precision%29)))

(fn ConstructionScript)