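; BP_Goal is the level goal: a coin-priced wall plus a win sphere that sends a flag interaction message.
; On BeginPlay it sets the displayed price to the BP_COINS count minus a small random amount.
; PayBox collects credits through a message to the overlapping actor, re-arming after partial payments.
; Full payment clears the game mode's CanChangeTime, runs a timeline scaling the wall's height, then hides the price text.
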(event OnComponentBeginOverlap(PayBox)
  (params (OverlappedComponent :type Primitive%20Component%20Object%20Reference) (OtherActor :type Actor%20Object%20Reference) (OtherComp :type Primitive%20Component%20Object%20Reference) (OtherBodyIndex :type Integer) (bFromSweep :type Boolean) (SweepResult :type Hit%20Result%20Structure%20%28by%20ref%29))
  (bind _wall (Variables|Default|GetWall))
  (bind _relativescale3d (Variables|/Script/Engine.SceneComponent|GetRelativeScale3D _wall))
  (Utilities|FlowControl|DoOnce false :!label _label
    (:Completed
      (bind _coins (Class|BPPlayerInteractions|PaythePrice(Message) OtherActor))
      (if (>= _coins (Variables|Default|GetPriceValue))
        (CallFunction|PayPriceValue _coins)
        (Variables|/Game/ThirdPerson/Blueprints/BP_ThirdPersonGameMode.BP_ThirdPersonGameMode_C|SetCanChangeTime (Variables|Default|GetGM) false)
        (bind _duration (Timeline|OpenDoor Play)
          (:Update
            (Transformation|SetRelativeScale3D _wall (Math|Vector|MakeVector (.x _relativescale3d) (.y _relativescale3d) (* _duration 3.0))))
          (:Finished
            (Rendering|SetVisibility (Variables|Default|GetTextRender) false false)))
        (else
          (CallFunction|PayPriceValue _coins)
          (Utilities|FlowControl|Delay 0.5)
          (goto _label Reset))))))

(event OnComponentBeginOverlap(WinSphere)
  (params (OverlappedComponent :type Primitive%20Component%20Object%20Reference) (OtherActor :type Actor%20Object%20Reference) (OtherComp :type Primitive%20Component%20Object%20Reference) (OtherBodyIndex :type Integer) (bFromSweep :type Boolean) (SweepResult :type Hit%20Result%20Structure%20%28by%20ref%29))
  (Class|BPPlayerInteractions|FlagInteraction(Message) OtherActor))

(event EventBeginPlay
  (bind _outactors (Actor|GetAllActorsOfClass "/Game/BPS/BP_COINS.BP_COINS_C"))
  (Variables|Default|SetPriceValue (- (Utilities|Array|Length _outactors) (Math|Random|RandomIntegerinRange 0 2)))
  (CallFunction|UpdateCostText)
  (bind _asbp_third_person_game_mode (Utilities|Casting|CastToBP_ThirdPersonGameMode (Game|GetGameMode)))
  (Variables|Default|SetGM _asbp_third_person_game_mode))

(event Collision|EventActorBeginOverlap
  (params (OtherActor :type Actor%20Object%20Reference)))

(event EventTick
  (params (DeltaSeconds :type Float%20%28single-precision%29)))

(fn ConstructionScript)

(fn UpdateCostText
  (Rendering|Components|TextRender|SetText (Variables|Default|GetTextRender) (Utilities|Text|ToText(Integer) (Variables|Default|GetPriceValue))))

(fn PayPriceValue
  (params (Credits :type Integer))
  (Variables|Default|SetPriceValue (Math|Integer|Clamp(Integer) (- (Variables|Default|GetPriceValue) Credits) 0 999))
  (CallFunction|UpdateCostText)
  (Audio|PlaySound2D "/Game/UI/Kenney/Sounds/Coins_Cue.Coins_Cue" 1.0 1.0 0.0 0 0))